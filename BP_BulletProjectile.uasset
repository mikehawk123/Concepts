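; Projectile actor that explodes on its first hit and carves away Paper2D sprite instances within the blast radius.
; After a zero-length delay at start, it applies its configurable local forward speed and collision radius.
; On destruction it spawns a radius-scaled BP_Explosion, then sphere-overlaps grouped sprite components to remove instances by distance.
; The removal loop repeats several times as a marked hack, as forward index removal can skip instances.
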(event `self.ReceiveBeginPlay`
  (`KismetSystemLibrary.Delay` 0.0)
  (`ProjectileMovementComponent.SetVelocityInLocalSpace` (`self.ProjectileMovement`) (`KismetMathLibrary.MakeVector` (`self.Projectile Speed`)))
  (`SphereComponent.SetSphereRadius` (`self.Sphere`) (`self.Projectile Radius`) true))

(event `self.ReceiveHit`
  (params (MyComp :type "PrimitiveComponent Object Reference") (Other :type "Actor Object Reference") (OtherComp :type "PrimitiveComponent Object Reference") (bSelfMoved :type Boolean) (HitLocation :type "Vector Structure") (HitNormal :type "Vector Structure") (NormalImpulse :type "Vector Structure") (Hit :type "HitResult Structure (by ref)"))
  (`/Engine/EditorBlueprintResources/StandardMacros.DoOnce` false
    (:`Completed`
      (`self.K2_DestroyActor`))))

(event `self.ReceiveDestroyed`
  (`|SpawnActorFromClass` "/Game/Blueprints/BP_Explosion.BP_Explosion_C" (`KismetMathLibrary.MakeTransform` (+ (`self.K2_GetActorLocation`) (0.0 100.0 0.0)) (struct) (`KismetMathLibrary.Conv_DoubleToVector` (/ (`self.Exposion Radius`) 50.0))) "AlwaysSpawn" "OverrideRootScale")
  (bind _outcomponents (`KismetSystemLibrary.SphereOverlapComponents` (`self.K2_GetActorLocation`) (`self.Exposion Radius`) (`self.Object Types`) "/Script/Paper2D.PaperGroupedSpriteComponent"))
  (for _array_element _outcomponents
    (`/Engine/EditorBlueprintResources/StandardMacros.IsValid` _array_element
      (:`Is Valid`
        (bind _aspaper_grouped_sprite_component (cast `PaperGroupedSpriteComponent` _array_element))
        (for _ (range 4)
          (for _index (range (+ (`PaperGroupedSpriteComponent.GetInstanceCount` _aspaper_grouped_sprite_component) 1))
            (if (< (`KismetMathLibrary.VSize` (- (.location (`PaperGroupedSpriteComponent.GetInstanceTransform` _aspaper_grouped_sprite_component _index true)) (`self.K2_GetActorLocation`))) (`self.Exposion Radius`))
              (`PaperGroupedSpriteComponent.RemoveInstance` _aspaper_grouped_sprite_component _index))))))))

(fn `UserConstructionScript`)